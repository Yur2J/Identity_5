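; Lobby player state that tracks a player's ready flag and nickname.
; It refreshes the first local player controller's BP_LobbyHUD when it begins play, is destroyed, or is marked ready through S2M_HandleReadyButton, which only sets the flag to true.
; CopyProperties passes the nickname on to a BP_PlayerState, carrying it beyond the lobby.
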(event `self.ReceiveBeginPlay`
  (`self.RefreshLobbyUI`)
  (add `Actor.OnDestroyed` (delegate `OnDestroyed_Event`)))

(event `OnDestroyed_Event`
  (params (DestroyedActor :type "Actor Object Reference"))
  (`self.RefreshLobbyUI`))

(event `S2M_HandleReadyButton`
  (set `self.bIsReady` true)
  (`self.RefreshLobbyUI`))

(event `self.ReceiveCopyProperties`
  (params (NewPlayerState :type "PlayerState Object Reference"))
  (`parent.ReceiveCopyProperties` NewPlayerState)
  (bind _asbp_player_state (cast `/Game/Blueprints/InGame/Character/BP_PlayerState` NewPlayerState))
  (set `/Game/Blueprints/InGame/Character/BP_PlayerState.Nickname` (`self.Nickname`) _asbp_player_state))

(fn `RefreshLobbyUI`
  (bind _returnvalue (`GameplayStatics.GetPlayerController` 0))
  (`/Engine/EditorBlueprintResources/StandardMacros.IsValid` _returnvalue
    (:`Is Valid`
      (bind _asbp_lobby_hud (cast `/Game/Blueprints/Lobby/BP_LobbyHUD` (`PlayerController.GetHUD` _returnvalue)))
      (`/Game/Blueprints/Lobby/BP_LobbyHUD.RefreshUI` _asbp_lobby_hud))))

(fn `UserConstructionScript`)