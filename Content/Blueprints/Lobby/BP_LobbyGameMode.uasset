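; Lobby game mode that assigns numbered nicknames to joining players and moves the session to the game level once everyone is ready.
; BeginPlay enables seamless travel and reads the target level name from the game instance.
; TryStartGame checks every lobby player state's ready flag, then waits briefly before running ServerTravel through a console command.
; The loading widget multicast is routed through the lobby GameState, as GameMode cannot host multicast RPCs.
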(event `TryStartGame`
  (if (`self.IsEverybodyReady`)
    (`KismetSystemLibrary.Delay` 1.0)
    ; Multicast RPC함수는 GameMode에서 정의 불가능! (GameState에서 정의해서 호출한다)
    (bind _asbp_lobby_game_state (cast `/Game/Blueprints/Lobby/BP_LobbyGameState` (`GameplayStatics.GetGameState`)))
    (`/Game/Blueprints/Lobby/BP_LobbyGameState.Multicast_ShowLoadingWidget` _asbp_lobby_game_state)
    (`KismetSystemLibrary.ExecuteConsoleCommand` (`KismetStringLibrary.Concat_StrStr` "ServerTravel " (`self.LevelName`)) null)))

(event `self.K2_PostLogin`
  (params (NewPlayer :type "PlayerController Object Reference"))
  ; 누군가 서버에 접속시 닉네임 설정
  (bind _asbp_lobby_player_state (cast `/Game/Blueprints/Lobby/BP_LobbyPlayerState` (`Controller.PlayerState` NewPlayer)))
  (bind _result (`/Engine/EditorBlueprintResources/StandardMacros.IncrementInt` (`self.NicknameIndex`))
    (:`  `
      (set `LobbyPlayerState.Nickname` (`|FormatText` "User{0}" _result) _asbp_lobby_player_state))))

(event `self.ReceiveBeginPlay`
  (set `self.bUseSeamlessTravel` true)
  (bind _asbp_game_instance (cast `/Game/Blueprints/BP_GameInstance` (`GameplayStatics.GetGameInstance`)))
  (set `self.LevelName` (`/Game/Blueprints/BP_GameInstance.LevelName` _asbp_game_instance)))

(fn `IsEverybodyReady`
  (returns (bIsReady :type Boolean))
  (for _array_element (`GameStateBase.PlayerArray` (`GameplayStatics.GetGameState`))
    (bind _asbp_lobby_player_state (cast `/Game/Blueprints/Lobby/BP_LobbyPlayerState` _array_element))
    (if (not (`/Game/Blueprints/Lobby/BP_LobbyPlayerState.bIsReady` _asbp_lobby_player_state))
      (return false)))
  (return true))

(fn `UserConstructionScript`)