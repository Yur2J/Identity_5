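; Lobby player controller that relays ready, nickname and role choices to the server through C2S/S2C events.
; Ready updates the player state and asks the lobby game mode to start; nicknames are written straight to the player state.
; Role selection reports duplicates via a placeholder print but still assigns the role; success refreshes the HUD and stores it in the GameInstance.
; The kick event is an empty stub.
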(event `HandleReadyButton`
  (`self.C2S_HandelReadyButton`))

(event `C2S_HandelReadyButton`
  (if (`KismetSystemLibrary.IsServer`)
    (bind _asbp_lobby_player_state (cast `/Game/Blueprints/Lobby/BP_LobbyPlayerState` (`Pawn.PlayerState` (`self.K2_GetPawn`))))
    (`/Game/Blueprints/Lobby/BP_LobbyPlayerState.S2M_HandleReadyButton` _asbp_lobby_player_state)
    (bind _asbp_lobby_game_mode (cast `/Game/Blueprints/Lobby/BP_LobbyGameMode` (`GameplayStatics.GetGameMode`)))
    (`/Game/Blueprints/Lobby/BP_LobbyGameMode.TryStartGame` _asbp_lobby_game_mode)))

(event `HandleChangeNickname`
  (params (Nickname :type Text))
  (`self.C2S_HandleChangeNickname` Nickname))

(event `S2C_KickedByServer`
  ; 강퇴로직X
)

(event `C2S_HandleChangeNickname`
  (params (Nickname :type Text))
  (bind _asbp_lobby_player_state (cast `/Game/Blueprints/Lobby/BP_LobbyPlayerState` (`Pawn.PlayerState` (`self.K2_GetPawn`))))
  (set `LobbyPlayerState.Nickname` Nickname _asbp_lobby_player_state))

(event `HandleSelectRole`
  (params (Role :type String))
  (`self.C2S_HandleSelectRole` Role))

(event `C2S_HandleSelectRole`
  (params (Role :type String))
  (for _array_element (`GameStateBase.PlayerArray` (`GameplayStatics.GetGameState`))
    (bind _asbp_lobby_player_state (cast `/Game/Blueprints/Lobby/BP_LobbyPlayerState` _array_element))
    (if (and (`KismetStringLibrary.EqualEqual_StrStr` (`/Game/Blueprints/Lobby/BP_LobbyPlayerState.SelectedRole` _asbp_lobby_player_state) Role) (!= _asbp_lobby_player_state (`self.PlayerState`)))
      (`self.S2C_RoleAlreadyTaken` Role)
      (else
        (`self.S2C_RoleSelectSuccess` Role))))
  (bind _asbp_lobby_player_state_2 (cast `/Game/Blueprints/Lobby/BP_LobbyPlayerState` (`self.PlayerState`)))
  (set `/Game/Blueprints/Lobby/BP_LobbyPlayerState.SelectedRole` Role _asbp_lobby_player_state_2)
  (`self.S2C_RoleSelectSuccess` Role))

(event `S2C_RoleAlreadyTaken`
  (params (Role :type String))
  ; 나중에 UI로 수정 (이미 선택한 역할버튼은 Set Enabled 설정해야됨)
  (`KismetSystemLibrary.PrintString` (`KismetTextLibrary.Conv_TextToString` (`|FormatText` "{Role}은 이미 선택된 역할입니다." Role)) true true (struct :`R` 1.0 :`A` 1.0) 5.0))

(event `S2C_RoleSelectSuccess`
  (params (Role :type String))
  (bind _asbp_lobby_hud (cast `/Game/Blueprints/Lobby/BP_LobbyHUD` (`self.GetHUD`)))
  (`/Game/Blueprints/Lobby/BP_LobbyHUD.RefreshUI` _asbp_lobby_hud)
  (bind _asbp_game_instance (cast `/Game/Blueprints/BP_GameInstance` (`GameplayStatics.GetGameInstance`)))
  (set `/Game/Blueprints/BP_GameInstance.SelectedRole` Role _asbp_game_instance))

(fn `UserConstructionScript`)