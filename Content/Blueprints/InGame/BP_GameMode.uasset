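; In-game GameMode that spawns players as Hunter or Survivor pawns.
; BeginPlay enables seamless travel and caches player 0's BP_PlayerState.
; SpawnPlayerCharacter switches on the given role, spawns the pawn at a hardcoded location and possesses it with the passed controller, defaulting to Survivor when no role is chosen.
; The role is saved to the cached PlayerState, so it always lands on player 0's, whichever controller is passed.
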(event `self.ReceiveBeginPlay`
  (`|ExecutionSequence`
    (:`then_0`
      ; Use Seamless Travel (Class Defaults 설정 O)
      (set `self.bUseSeamlessTravel` true))
    (:`then_1`
      ; PlayerState Ref 저장
      (bind _asbp_player_state (cast `/Game/Blueprints/InGame/BP_PlayerState` (`GameplayStatics.GetPlayerState` 0)))
      (set `self.InGamePSRef` _asbp_player_state))))

(fn `SpawnPlayerCharacter`
  (params (InController :type "PlayerController Object Reference") (Role :type String))
  (switch `string` Role
    (:`Default`
      ; 선택한 역할로 Spawn 후 Possess
      ;; 역할 선택 안 했을 경우 (Default) 처리해야 함
      (`KismetSystemLibrary.PrintString` "역할이 선택되지 않았습니다. 생존자 모드로 시작합니다." true true (struct :`R` 1.0 :`A` 1.0) 5.0)
      (bind _returnvalue (`|SpawnActorFromClass` "/Game/Blueprints/InGame/Character/BP_Survivor.BP_Survivor_C" (`KismetMathLibrary.MakeTransform` (-680.0 -2620.0 192.0)) "Undefined" "MultiplyWithRoot" null null))
      (`Controller.Possess` InController _returnvalue)
      ; PlayerState에 무슨 역할 선택했는지 저장
      (set `/Game/Blueprints/InGame/BP_PlayerState.SelectedRole` "Survivor" (`self.InGamePSRef`)))
    (:`Hunter`
      (bind _returnvalue_2 (`|SpawnActorFromClass` "/Game/Blueprints/InGame/Character/BP_Hunter.BP_Hunter_C" (`KismetMathLibrary.MakeTransform` (-2090.0 1930.0 220.0)) "Undefined" "MultiplyWithRoot" null null))
      (`Controller.Possess` InController _returnvalue_2)
      (set `/Game/Blueprints/InGame/BP_PlayerState.SelectedRole` "Hunter" (`self.InGamePSRef`)))
    (:`Survivor`
      (bind _returnvalue_3 (`|SpawnActorFromClass` "/Game/Blueprints/InGame/Character/BP_Survivor.BP_Survivor_C" (`KismetMathLibrary.MakeTransform` (-680.0 -2620.0 220.0)) "Undefined" "MultiplyWithRoot" null null))
      (`Controller.Possess` InController _returnvalue_3)
      (set `/Game/Blueprints/InGame/BP_PlayerState.SelectedRole` "Survivor" (`self.InGamePSRef`)))))

(fn `UserConstructionScript`)