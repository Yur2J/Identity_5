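; Game state for a Hunter-versus-Survivor match, handling the game-over screen and decoder-based exit progress.
; C2M_OnGameEnded latches GameHasEnded, then uses the local player's SelectedRole and the winner to show a win or lose widget with UI-only input.
; OnDecoderCompleted acts only if ExitUnlocked is already true: it shows the prompt widget's unlock notice, counts the decoder, and sets ExitUnlocked at the threshold.
; The exit-unlock RepNotify is empty.
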(event `C2M_OnGameEnded`
  (params (InWinner :type "/Game/Blueprints/InGame/Enum/E_WinnerType Enum" :default "NewEnumerator0"))
  (bind _returnvalue (`GameplayStatics.GetPlayerController` 0))
  (bind _returnvalue_2 (`GameplayStatics.GetPlayerController` 0))
  (bind _returnvalue_3 (`GameplayStatics.GetPlayerController` 0))
  (bind _returnvalue_4 (`GameplayStatics.GetPlayerController` 0))
  (bind _returnvalue_5 (`GameplayStatics.GetPlayerController` 0))
  (`/Engine/EditorBlueprintResources/StandardMacros.IsValid` _returnvalue_2
    (:`Is Valid`
      (bind _asbp_player_state (cast `/Game/Blueprints/InGame/BP_PlayerState` (`Controller.PlayerState` _returnvalue_2)))
      (if (not (`self.bGameHasEnded`))
        (set `self.bGameHasEnded` true)
        (switch `string` (`/Game/Blueprints/InGame/BP_PlayerState.SelectedRole` _asbp_player_state)
          (:`Hunter`
            ; BP_Hunter에서 IsHooking후 실행
            (if (`|EnumEquality` InWinner "NewEnumerator2")
              ; 거꾸로 되어있음 문제 파악 ㄱ
              (bind _returnvalue_6 (`|CreateWidget` "/Game/Assets/UI/Widget/InGame/WBP_Hunter_Lose.WBP_Hunter_Lose_C" _returnvalue_3))
              (`UserWidget.AddToViewport` _returnvalue_6 0)
              (`WidgetBlueprintLibrary.SetInputMode_UIOnlyEx` _returnvalue_3 null)
              (set `PlayerController.bShowMouseCursor` true _returnvalue_3)
              (else
                (bind _returnvalue_7 (`|CreateWidget` "/Game/Assets/UI/Widget/InGame/WBP_Hunter_Win.WBP_Hunter_Win_C" _returnvalue))
                (`UserWidget.AddToViewport` _returnvalue_7 0)
                (`WidgetBlueprintLibrary.SetInputMode_UIOnlyEx` _returnvalue null)
                (set `PlayerController.bShowMouseCursor` true _returnvalue))))
          (:`Survivor`
            (if (`|EnumEquality` InWinner "NewEnumerator5")
              (bind _returnvalue_8 (`|CreateWidget` "/Game/Assets/UI/Widget/InGame/WBP_Survivor_Lose.WBP_Survivor_Lose_C" _returnvalue_4))
              (`UserWidget.AddToViewport` _returnvalue_8 0)
              (`WidgetBlueprintLibrary.SetInputMode_UIOnlyEx` _returnvalue_4 null)
              (set `PlayerController.bShowMouseCursor` true _returnvalue_4)
              (else
                (bind _returnvalue_9 (`|CreateWidget` "/Game/Assets/UI/Widget/InGame/WBP_Survivor_Win.WBP_Survivor_Win_C" _returnvalue_5))
                (`UserWidget.AddToViewport` _returnvalue_9 0)
                (`WidgetBlueprintLibrary.SetInputMode_UIOnlyEx` _returnvalue_5 null)
                (set `PlayerController.bShowMouseCursor` true _returnvalue_5)))))))))

(fn `OnDecoderCompleted`
  (if (`self.bExitUnlocked`)
    (bind _foundwidgets (`WidgetBlueprintLibrary.GetAllWidgetsOfClass` "/Game/Assets/UI/Widget/InGame/WBP_InteractPrompt.WBP_InteractPrompt_C"))
    (bind _output (`|GetArrayItem` _foundwidgets))
    (`/Engine/EditorBlueprintResources/StandardMacros.IsValid` _output
      (:`Is Valid`
        (`/Game/Assets/UI/Widget/InGame/WBP_InteractPrompt.ShowExitUnlockedNotification` _output)
        (set `self.CompletedDecoderCount ` (+ (`self.CompletedDecoderCount `) 1))
        (if (>= (`self.CompletedDecoderCount `) 3)
          (set `self.bExitUnlocked` true))))))

(fn `OnRep_bExitUnlocked`)

(fn `UserConstructionScript`)