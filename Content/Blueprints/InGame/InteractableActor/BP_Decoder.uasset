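; BP_Decoder is an interactable decoder that players progress to completion, with its state updated on the server.
; Start and stop functions control a looping timer that drives TickDecode, which adds FillRate-scaled progress on authority only.
; A failed skill check knocks progress back.
; At full progress it marks itself completed, clears the timer and notifies BP_GameState through OnDecoderCompleted.
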(event `self.ReceiveBeginPlay`
  (`/Engine/EditorBlueprintResources/ActorMacros.Switch Has Authority`
    (:`Authority`
      (set `self.bIsCompleted` false)
      (set `self.DecodeProgress` 0.0)
      (set `self.bBeingDecoded` false)
      (`KismetSystemLibrary.K2_ClearAndInvalidateTimerHandle` (`self.DecodeTimerHandle `)))))

(event `TickDecode`
  ; Local Event (not RPC)
  (`/Engine/EditorBlueprintResources/ActorMacros.Switch Has Authority`
    (:`Authority`
      (bind _output_get (set `self.DecodeProgress` (`KismetMathLibrary.FClamp` (+ (`self.DecodeProgress`) (* (`self.FillRate`) 0.2)) 0.0 100.0)))
      (if (>= _output_get 100.0)
        (set `self.bIsCompleted` true)
        (set `self.bBeingDecoded` false)
        (`KismetSystemLibrary.K2_ClearAndInvalidateTimerHandle` (`self.DecodeTimerHandle `))
        (bind _asbp_game_state (cast `/Game/Blueprints/InGame/BP_GameState` (`GameplayStatics.GetGameState`))
          (:`then`
            (`/Game/Blueprints/InGame/BP_GameState.OnDecoderCompleted` _asbp_game_state))
          (:`CastFailed`
            (`KismetSystemLibrary.PrintString` "해독기에서 GS캐스팅 실패")))))))

(fn `ApplySkillCheckFail`
  (set `self.DecodeProgress` (`KismetMathLibrary.FClamp` (- (`self.DecodeProgress`) 10.0) 0.0 100.0)))

(fn `ServerStartDecoding`
  (if (and (not (`self.bIsCompleted`)) (not (`self.bBeingDecoded`)))
    (set `self.bBeingDecoded` true)
    (bind _returnvalue (`KismetSystemLibrary.K2_SetTimerDelegate` (`|CreateDelegate` :!event `TickDecode`) 0.2 true))
    (set `self.DecodeTimerHandle ` _returnvalue)))

(fn `ServerStopDecoding`
  (`KismetSystemLibrary.K2_ClearAndInvalidateTimerHandle` (`self.DecodeTimerHandle `))
  (set `self.bBeingDecoded` false))

(fn `UserConstructionScript`)