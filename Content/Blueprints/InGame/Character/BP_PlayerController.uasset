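; In-game player controller that sets up local input and requests a character spawn for the player's chosen role (watcher or survivor).
; On BeginPlay, only the local controller adds the default Enhanced Input mapping context and switches to game-only input.
; It then passes the role stored in BP_GameInstance through a client-to-server spawn event, which delegates spawning to BP_GameMode.
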(event `self.ReceiveBeginPlay`
  (bind _returnvalue (pcsubsystem `EnhancedInputLocalPlayerSubsystem` self))
  (if (`self.IsLocalPlayerController`)
    (`|ExecutionSequence`
      (:`then_0`
        ; Enhanced Input (Subsystem)
        (`/Engine/EditorBlueprintResources/StandardMacros.IsValid` _returnvalue
          (:`Is Valid`
            (`EnhancedInputSubsystemInterface.AddMappingContext` _returnvalue "/Game/Input/IMC_Default.IMC_Default" 0 (struct))
            (`WidgetBlueprintLibrary.SetInputMode_GameOnly` self))))
      (:`then_1`
        ; GameInstance에서 감시자/생존자 모드 선택해서 Spawn - Possess
        (bind _asbp_game_instance (cast `/Game/Blueprints/BP_GameInstance` (`GameplayStatics.GetGameInstance`))
          (:`then`
            (`self.C2S_RequestSpawn` (`/Game/Blueprints/BP_GameInstance.SelectedRole` _asbp_game_instance)))
          (:`CastFailed`
            (`KismetSystemLibrary.PrintString` "InGamePC에서 GameInstance캐스팅 실패" true true (struct :`G` 0.66 :`B` 1.0 :`A` 1.0) 999.0)))))))

(event `C2S_RequestSpawn`
  (params (Role :type String))
  (bind _asbp_game_mode (cast `/Game/Blueprints/InGame/BP_GameMode` (`GameplayStatics.GetGameMode`))
    (:`then`
      (`/Game/Blueprints/InGame/BP_GameMode.SpawnPlayerCharacter` _asbp_game_mode self Role))
    (:`CastFailed`
      (`KismetSystemLibrary.PrintString` "InGamePC에서 GameMode캐스팅 실패" true true (struct :`G` 0.66 :`B` 1.0 :`A` 1.0) 999.0))))

(fn `UserConstructionScript`)