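; BP_PlayerState is a player state Blueprint with Nickname and SelectedRole variables, apparently meant to carry them over to a newly created PlayerState.
; The CopyProperties event is currently empty, so this graph copies neither value.
; The disconnected logic calls the parent, casts the new state to BP_PlayerState, copies both values and prints them, or prints a failure message if the cast fails.
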(event `self.ReceiveCopyProperties`
  (params (NewPlayerState :type "PlayerState Object Reference"))
  ; 새로 태어난 PlayerState변수에 값 새로 넣음
)

(fn `UserConstructionScript`)